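; SoldierAI is an AI controller that sends its AI_Character wandering between the Waypoint actors it is allowed to visit.
; On BeginPlay it gathers waypoints whose AllowedAccess list contains the pawn, shuffles them and moves to the first.
; Each completed move, whatever its result, repeats the search after a short delay, appending to Routes without clearing it, so entries accumulate.
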(event Custom|ReceiveMoveCompleted_Event_0
  (params (RequestID :type AI%20Request%20ID%20Structure) (Result :type EPathFollowingResult%20Enum :default "Success"))
  (bind _routes (Variables|Default|GetRoutes))
  (Utilities|FlowControl|Delay 3.0)
  (bind _outactors (Actor|GetAllActorsOfClass "/Game/Blueprint/Waypoint.Waypoint_C"))
  (bind _asai_character (Utilities|Casting|CastToAI_Character (Pawn|GetControlledPawn)))
  (for _array_element _outactors
    (if (!= (Utilities|Array|FindItem (Variables|/Game/Blueprint/Waypoint.Waypoint_C|GetAllowedAccess _array_element) _asai_character) -1)
      (Utilities|Array|Add (Variables|Default|GetRoutes) _array_element)))
  (Utilities|Array|Shuffle _routes)
  (AI|Navigation|MovetoActor (Utilities|Array|Get(acopy) _routes) -1.0 true true))

(event EventBeginPlay
  (bind _routes (Variables|Default|GetRoutes))
  (EventDispatchers|BindEventtoReceiveMoveCompleted (delegate Custom|ReceiveMoveCompleted_Event_0))
  (bind _outactors (Actor|GetAllActorsOfClass "/Game/Blueprint/Waypoint.Waypoint_C"))
  (bind _asai_character (Utilities|Casting|CastToAI_Character (Pawn|GetControlledPawn)))
  (for _array_element _outactors
    (if (!= (Utilities|Array|FindItem (Variables|/Game/Blueprint/Waypoint.Waypoint_C|GetAllowedAccess _array_element) _asai_character) -1)
      (Utilities|Array|Add (Variables|Default|GetRoutes) _array_element)))
  (Utilities|Array|Shuffle _routes)
  (AI|Navigation|MovetoActor (Utilities|Array|Get(acopy) _routes) -1.0 true true))

(fn ConstructionScript)